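; Door actor Blueprint that swings open and closed in response to its DoorRotation component's OnOpen and OnClose events.
; A timeline drives a yaw angle, combined with the rotation saved at BeginPlay, and plays forward to open and in reverse to close.
; An event track on the timeline plays the door lock sound at the actor's location.
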(event `self.ReceiveBeginPlay`
  (set `self.intial Rotation` (`self.K2_GetActorRotation`)))

(event `self.DoorRotation.OnOpen`
  (bind (_direction _openangle) (`Timeline|OpenDoor` :!label _label)
    (:`Update`
      (`self.K2_SetActorRotation` (`KismetMathLibrary.ComposeRotators` (`KismetMathLibrary.MakeRotator` 0.0 0.0 _openangle) (`self.intial Rotation`))))
    (:`Sound Timing`
      (`GameplayStatics.PlaySoundAtLocation` "/Game/Audio/door-lock.door-lock" (`self.K2_GetActorLocation`)))))

(event `self.DoorRotation.OnClose`
  (goto _label :!via `Reverse`))

(fn `UserConstructionScript`)